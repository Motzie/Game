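; AddHealthBP is a healing actor that gradually restores the player character's health while something overlaps it.
; Begin overlap sets an IsIn flag and starts a Delay-driven loop that adds a small amount of Health several times a second, clamped to MaxHealth.
; End overlap clears the flag to stop the loop.
; The overlapping actor is not checked; healing always targets player 0's ThirdPersonCharacter.
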(event Collision|EventActorBeginOverlap
  (params (OtherActor :type Actor%20Object%20Reference))
  (Variables|Default|SetIsIn true)
  (if (Variables|Default|GetIsIn) :!label _label
    (bind _asthird_person_character (Utilities|Casting|CastToThirdPersonCharacter (Game|GetPlayerCharacter 0)))
    (Variables|/Game/ThirdPersonBP/Blueprints/ThirdPersonCharacter.ThirdPersonCharacter_C|SetHealth _asthird_person_character (Math|Float|Clamp(Float) (+ (Variables|/Game/ThirdPersonBP/Blueprints/ThirdPersonCharacter.ThirdPersonCharacter_C|GetHealth _asthird_person_character) 1.0) 0.0 (Variables|/Game/ThirdPersonBP/Blueprints/ThirdPersonCharacter.ThirdPersonCharacter_C|GetMaxHealth _asthird_person_character)))
    (Utilities|FlowControl|Delay 0.2)
    (goto _label)))

(event Collision|EventActorEndOverlap
  (params (OtherActor :type Actor%20Object%20Reference))
  (Variables|Default|SetIsIn false))

(fn ConstructionScript)